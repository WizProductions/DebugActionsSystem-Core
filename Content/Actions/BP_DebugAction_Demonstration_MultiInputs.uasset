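; Demonstration debug action, titled "PrintFloatValue", that shows how one action uses multiple debug inputs.
; When its parent folder is developed, it requests a ranged float slider and a Blueprint-made text input, set as password, from the debug subsystem.
; Both requests use the default shared key tag, so other actions requesting the same class and tag share those inputs.
; On execute, it validates both inputs, prints their values on screen and returns success.
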(fn `GetDebugActionTitle`
  (returns (ReturnValue :type Text))
  ;[0 0.5694 0.613] The title in the button for the debug action
  (return "PrintFloatValue"))

(fn `OnExecuteDebugAction`
  (returns (ReturnValue :type "EDebugActionResult Enum"))
  (bind _myfloatslider (`self.MyFloatSlider`))
  (bind _mytextet (`self.MyTextET`))
  ;[0.4739 0.3827 0.01125] Get the value and execute what you want, input cannot be invalid if the system is correctly enabled and used
  (`/Engine/EditorBlueprintResources/StandardMacros.IsValid` _myfloatslider
    (:`Is Valid`
      (`/Engine/EditorBlueprintResources/StandardMacros.IsValid` _mytextet
        (:`Is Valid`
          (`KismetSystemLibrary.PrintString` (`self.MyDebugSubsystem`) (`KismetStringLibrary.Concat_StrStr` "Value of slider: " (`KismetStringLibrary.Conv_DoubleToString` (`DebugInput_FloatSlider.GetValue` _myfloatslider)) " \nValue of Text input: " (`KismetTextLibrary.Conv_TextToString` (`/DebugActionsSystemCore/Inputs/DebugInput_TextET.GetValue` _mytextet))) true true (struct :`R` 1.0 :`G` 1.0 :`A` 1.0) 7.0)
          (return "Success"))))))

(fn `OnParentFolderIsDeveloped`
  (params (ParentFolder :type "DebugActionFolder Object Reference"))
  ;[0 0.1097 0.4913] Request the debug input you want for this action (as much as you want in the limit of number of debug input slot added in panel)
  (bind _outdebuginput (`DebugSubsystem.RequestDebugInput` (`self.MyDebugSubsystem`) "/Script/DebugActionsSystemCore.DebugInput_FloatSlider" (struct :`TagName` "DAS.SharedDIKey.Default"))) ; Request a shared debug input by default key tag other action request this input class with this same key tag get exactly the same input
  (bind _output_get (set `self.MyFloatSlider` _outdebuginput))
  ;[0.4356 0.4391 0] In this case, optional setup, but recommended to configure more things (Min/Max, specific input title...)
  (`DebugInput_FloatSlider.Setup` _output_get "FloatInput" (make `Vector2f` -150.0 150.0) 0.0)
  ;[0.2483 0.4851 0.4913] 2nd request of input with setup
  (bind _outdebuginput_2 (`DebugSubsystem.RequestDebugInput` (`self.MyDebugSubsystem`) "/DebugActionsSystemCore/Inputs/DebugInput_TextET.DebugInput_TextET_C" (struct :`TagName` "DAS.SharedDIKey.Default"))) ; Same request with text debug input created in Blueprint.
  (bind _output_get_2 (set `self.MyTextET` _outdebuginput_2))
  (`/DebugActionsSystemCore/Inputs/DebugInput_TextET.Setup` _output_get_2 "StringInput" true))