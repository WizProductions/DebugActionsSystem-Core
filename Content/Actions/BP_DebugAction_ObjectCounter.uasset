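; BP_DebugAction_ObjectCounter is a debug action that counts the instances of a selected actor class in the world.
; When its parent folder is developed, it requests an unshared class selector input, so each action gets its own, filtered by its configured top actor class.
; On execute, it runs GetAllActorsOfClass on the selection and prints the count, or prints an error and fails when no class is selected.
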(fn `GetDebugActionTitle`
  (returns (ReturnValue :type Text))
  ;[0 0.5694 0.613] The title in the button for the debug action (Customizable in DebugAction settings in the Data Asset)
  (return (`self.DebugActionTitle`)))

(fn `OnExecuteDebugAction`
  (returns (ReturnValue :type "EDebugActionResult Enum"))
  (bind _myunsharedclassselector (`self.MyUnsharedClassSelector`))
  (bind _returnvalue (`DebugInput_ClassSelector.GetValue` _myunsharedclassselector))
  ;[0.4318 0.5174 0.1439] Get instance/object count of selected actor class
  (`/Engine/EditorBlueprintResources/StandardMacros.IsValid` _myunsharedclassselector
    (:`Is Valid`
      (bind _asactor (castclass `Actor` _returnvalue)
        (:`then`
          (bind _outactors (`GameplayStatics.GetAllActorsOfClass` (`self.MyDebugSubsystem`) _asactor))
          (`KismetSystemLibrary.PrintString` (`self.MyDebugSubsystem`) (`KismetStringLibrary.Concat_StrStr` (`KismetStringLibrary.Conv_IntToString` (`KismetArrayLibrary.Array_Length` _outactors)) " object(s) of class: " (`KismetSystemLibrary.GetClassDisplayName` _returnvalue) " found.") true true (struct :`R` 1.0 :`G` 1.0 :`A` 1.0) 7.0)
          (return "Success"))
        (:`CastFailed`
          ;[0.613 0.2733 0.06689] Catch if no class selected.
          (`KismetSystemLibrary.PrintString` (`self.MyDebugSubsystem`) "No class selected for my class filter." true true (struct :`R` 1.0 :`G` 0.000277 :`A` 1.0) 7.0)
          (return "Fail"))))))

(fn `OnParentFolderIsDeveloped`
  (params (ParentFolder :type "DebugActionFolder Object Reference"))
  ;[0 0.2327 0.5] Request an Unshared debug input, the tag UnShared is special and the input requested with the tag is reserved for an instance of the action requester.
  ;
  ; An input is shared by his class and by the tag in the request.
  ; For example, OpenLevel & SeamlessTravel share the same input because both wants a levelname and can were not designed to be used at the same time.
  ;
  ; I strongly recommend choosing a shared tag each time or creating one if necessary. Inputs are organized using tags and folders. If there are too many inputs, they will no longer appear.
  ; This is just an example; the UnShared tag is not recommended.
  ;
  ; For the current example, the ObjectCounter, we prefer to have one input for each action because each action depends solely on the parameters of the ObjectCounter action.
  (bind _outdebuginput (`DebugSubsystem.RequestDebugInput` (`self.MyDebugSubsystem`) "/Script/DebugActionsSystemCore.DebugInput_ClassSelector" (struct :`TagName` "DAS.SharedDIKey.UnShared")))
  (bind _output_get (set `self.MyUnsharedClassSelector` _outdebuginput))
  (`DebugInput_ClassSelector.Setup` _output_get (`self.DebugInputTItle`) (`self.TopActorClass`) (`self.Include Parent Class`) (`self.Include Abstract Class`) true))